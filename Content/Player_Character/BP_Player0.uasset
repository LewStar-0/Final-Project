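; Click-to-move player character that fights enemies and bosses, toggles its inventory with Tab, and reloads or opens the Dungeon level when health runs out.
; Mouse clicks line-trace under the cursor: left moves to Terrain-tagged hits or attempts melee, right attempts ranged.
; Attack accepts BP_Enemy or BP_Boss, turns to face it, checks range, then plays an animation and applies typed damage directly.
; The ranged distance check has no target connected.
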(event `Key|Tab`
  (params (Key :type "Key Structure"))
  (bind _ac_inventorycomponent (`self.AC_InventoryComponent`))
  ;[1 1 1] Handle inventory interface
  (:`Pressed`
    (`/Engine/EditorBlueprintResources/StandardMacros.FlipFlop`
      (:`A`
        (`/Game/InventoryComponet/AC_InventoryComponent.F_ShowInventory` _ac_inventorycomponent))
      (:`B`
        (`/Game/InventoryComponet/AC_InventoryComponent.F Hide Inventory` _ac_inventorycomponent)))))

(event `Key|LeftMouseButton`
  (params (Key :type "Key Structure"))
  (bind (_worldlocation _worlddirection) (`PlayerController.DeprojectMousePositionToWorld` (`GameplayStatics.GetPlayerController` 0)))
  ;[1 1 1] Get The location under the mouse click
  (:`Pressed`
    (bind (_outhit _returnvalue) (`KismetSystemLibrary.LineTraceSingle` _worldlocation (+ _worldlocation (* _worlddirection 10000.0)) "TraceTypeQuery1"))
    ;[1 1 1] Validate the hit
    (if _returnvalue
      (bind (_bblockinghit _binitialoverlap _time _distance _location _impactpoint _normal _impactnormal _physmat _hitactor) (`GameplayStatics.BreakHitResult` _outhit))
      ;[1 1 1] Check if the hit object was a terrain piece, move if it was
      (if (`self.ActorHasTag` _hitactor "Terrain")
        (`AIBlueprintHelperLibrary.SimpleMoveToLocation` (`self.GetController`) _location)))))

(event `self.ReceiveAnyDamage`
  (params (Damage :type "Float (single-precision)") (DamageType :type "DamageType Object Reference") (InstigatedBy :type "Controller Object Reference") (DamageCauser :type "Actor Object Reference"))
  ;[1 1 1] Handle Damage
  (set `self.Health` (- (`self.Health`) Damage))
  (if (<= (`self.Health`) 0.0)
    (`GameplayStatics.OpenLevel` "Dungeon")
    (else
      ;[1 1 1] Print for testing DELETE LATER
      (`KismetSystemLibrary.PrintString` "OW!!!!!"))))

(event `Key|LeftMouseButton`
  (params (Key :type "Key Structure"))
  (bind (_worldlocation _worlddirection) (`PlayerController.DeprojectMousePositionToWorld` (`GameplayStatics.GetPlayerController` 0)))
  ;[1 1 1] Check if you clicked and enemy, if you u did then attack
  (:`Pressed`
    (bind _outhit (`KismetSystemLibrary.LineTraceSingle` _worldlocation (+ _worldlocation (* _worlddirection 10000.0)) "TraceTypeQuery1"))
    (`self.Attack` (`.HitActor` (`GameplayStatics.BreakHitResult` _outhit)))))

(event `Key|RightMouseButton`
  (params (Key :type "Key Structure"))
  (bind (_worldlocation _worlddirection) (`PlayerController.DeprojectMousePositionToWorld` (`GameplayStatics.GetPlayerController` 0)))
  ;[1 1 1] check for an enemy to range attack on
  (:`Pressed`
    (bind _outhit (`KismetSystemLibrary.LineTraceSingle` _worldlocation (+ _worldlocation (* _worlddirection 10000.0)) "TraceTypeQuery1"))
    (`self.Attack` (`.HitActor` (`GameplayStatics.BreakHitResult` _outhit)) 1)))

(fn `Attack`
  (params (Target :type "Actor Object Reference") (AttackType :type Integer))
  (bind _mesh (`self.Mesh`))
  (bind _mesh_2 (`self.Mesh`))
  (bind (_returnvalue_roll _returnvalue_pitch _returnvalue_yaw) (`KismetMathLibrary.BreakRotator` (`KismetMathLibrary.FindLookAtRotation` (`self.K2_GetActorLocation`) (`self.K2_GetActorLocation` Target))))
  ;[1 1 1] Validate that it's an enemy
  (cast `/Game/Enemies/BP_Enemy` Target
    (:`then`
      _)
    (:`CastFailed`
      (cast `/Game/Enemies/BP_Boss` Target)))
  ;[1 1 1] Rotate to face the enemy
  (`self.K2_SetActorRotation` (`KismetMathLibrary.MakeRotator` 0.0 0.0 _returnvalue_yaw))
  ;[1 1 1] Determine attack type
  (switch `int` AttackType
    (:`0`
      ;[1 1 1] Handle a Mellee Attack
      (if (<= (`self.GetDistanceTo` Target) (`self.MelleeAttackDistance`))
        (`SkeletalMeshComponent.PlayAnimation` _mesh "/Game/Anims/Player_MeleeAttack.Player_MeleeAttack" false)
        (`GameplayStatics.ApplyDamage` Target 10.0 null null "/Game/BP_MelleeDamage.BP_MelleeDamage_C")
        (`SkeletalMeshComponent.PlayAnimation` _mesh "/Game/Anims/Player_Walk.Player_Walk" true)
        ;[1 1 1] Print Attack, TESTING DELETE LATER
        (`KismetSystemLibrary.PrintString` "Mellee attack")
        (`KismetSystemLibrary.PrintString` (`KismetSystemLibrary.GetDisplayName` Target))))
    (:`1`
      ;[1 1 1] Handle a Ranged Attack
      (if (<= (`self.GetDistanceTo` null) (`self.RangedAttackDistance`))
        (`SkeletalMeshComponent.PlayAnimation` _mesh_2 "/Game/Anims/Player_RangedAttack.Player_RangedAttack" false)
        (`GameplayStatics.ApplyDamage` Target 10.0 null null "/Game/BP_RangedDamage.BP_RangedDamage_C")
        (`SkeletalMeshComponent.PlayAnimation` _mesh_2 "/Game/Anims/Player_Walk.Player_Walk" true)
        (`KismetSystemLibrary.PrintString` "Ranged attack")
        (`KismetSystemLibrary.PrintString` (`KismetSystemLibrary.GetDisplayName` Target))))))

(fn `UserConstructionScript`)
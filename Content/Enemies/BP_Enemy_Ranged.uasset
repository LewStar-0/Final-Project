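; BP_Enemy_Ranged is an enemy that damages its Target and can itself be killed.
; Every Tick calls Attack, which applies fixed damage directly to a valid Target, then sets a game-time cooldown of a few seconds.
; Despite the name, it has no range check or projectile, and Target is not assigned in these graphs.
; AnyDamage subtracts from Health and destroys the actor at zero or below.
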(event `Attack`
  ;[1 1 1] Check attack cooldown
  (if (>= (`KismetSystemLibrary.GetGameTimeInSeconds`) (`self.AttackCooldown`))
    ;[1 1 1] Check if we have a valid target
    (`/Engine/EditorBlueprintResources/StandardMacros.IsValid` (`self.Target`)
      (:`Is Valid`
        ;[1 1 1] Attack
        (`GameplayStatics.ApplyDamage` (`self.Target`) 10.0)
        ;[1 1 1] Reset the attack cooldown
        (set `self.AttackCooldown` (+ (`KismetSystemLibrary.GetGameTimeInSeconds`) 3.0))))))

(event `self.ReceiveAnyDamage`
  (params (Damage :type "Float (single-precision)") (DamageType :type "DamageType Object Reference") (InstigatedBy :type "Controller Object Reference") (DamageCauser :type "Actor Object Reference"))
  ;[1 1 1] Set health
  (set `self.Health` (- (`self.Health`) Damage))
  ;[1 1 1] Check for death
  (if (<= (`self.Health`) 0.0)
    (`self.K2_DestroyActor`)))

(event `self.ReceiveTick`
  (params (DeltaSeconds :type "Float (single-precision)"))
  (`parent.ReceiveTick` DeltaSeconds)
  (`self.Attack`))

(fn `UserConstructionScript`
  (`parent.UserConstructionScript`))
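; Enemy actor that chases the player when they come within aggro range.
; Each tick it caches the first BP_Player0 found as its Target if none is valid, then runs movement.
; Inside AggroRange it uses SimpleMoveToLocation to approach until closer than CombatRange, then moves to its own location to hold position.
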(event `self.ReceiveTick`
  (params (DeltaSeconds :type "Float (single-precision)"))
  ;[1 1 1] Get a reference to the player, if needed
  (`self.GetRefToPlayer`)
  ;[1 1 1] Move
  (`self.MoveTowardsPlayer`))

(fn `GetRefToPlayer`
  (`/Engine/EditorBlueprintResources/StandardMacros.IsValid` (`self.Target`)
    (:`Is Not Valid`
      (bind _outactors (`GameplayStatics.GetAllActorsOfClass` "/Game/Player_Character/BP_Player0.BP_Player0_C"))
      (set `self.Target` (`|GetArrayItem` _outactors)))))

(fn `MoveTowardsPlayer`
  ;[1 1 1] check if the ref to player is valid
  (`/Engine/EditorBlueprintResources/StandardMacros.IsValid` (`self.Target`)
    (:`Is Valid`
      ;[1 1 1] check if the player is within aggro range
      (if (<= (`self.GetDistanceTo` (`self.Target`)) (`self.AggroRange`))
        ;[1 1 1] Check if the player is within range
        (if (>= (`self.GetDistanceTo` (`self.Target`)) (`self.Combat Range`))
          ;[1 1 1] Move towards the player if not at the optimal range
          (`AIBlueprintHelperLibrary.SimpleMoveToLocation` (`self.GetController`) (`self.K2_GetActorLocation` (`self.Target`)))
          (else
            ;[1 1 1] Stay at location if at the right range
            (`AIBlueprintHelperLibrary.SimpleMoveToLocation` (`self.GetController`) (`self.K2_GetActorLocation`))))))))

(fn `UserConstructionScript`)
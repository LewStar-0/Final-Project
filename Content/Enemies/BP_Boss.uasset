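; Boss enemy that targets the first BP_Player0 found and attempts an attack every Tick, gated by a game-time cooldown.
; The Healthbar value selects the phase: melee only, then alternating with minion spawns, then adding ranged, rotated by an attack counter; nothing here updates Healthbar.
; Melee and ranged share identical move-or-damage logic, while spawning drops melee, ranged and flying minions nearby.
; Incoming damage reduces Health and destroys the boss at zero.
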(event `Attack`
  ;[1 1 1] Run all checks before attacking
  (if (>= (`KismetSystemLibrary.GetGameTimeInSeconds`) (`self.AttackCooldown`))
    (`/Engine/EditorBlueprintResources/StandardMacros.IsValid` (`self.TargetPlayer`)
      (:`Is Valid`
        ;[1 1 1] execute attacks based on what healthbar you're on
        ;;[1 1 1] Select Phase
        (switch `int` (`self.Healthbar`)
          (:`0`
            (`self.Melee Attack` :!label _label))
          (:`1`
            (goto _label))
          (:`2`
            (switch `int` (mod (`self.AttackIndex(Accumulator)`) 2) :!label _label_2
              (:`Default`
                (`self.Spawn Enemies` :!label _label_3))
              (:`0`
                (`self.Melee Attack`))
              (:`1`
                (goto _label_3))))
          (:`3`
            (goto _label_2))
          (:`4`
            (switch `int` (mod (`self.AttackIndex(Accumulator)`) 3) :!label _label_4
              (:`Default`
                (`self.Ranged Attack` :!label _label_5))
              (:`0`
                (`self.Melee Attack`))
              (:`1`
                (`self.Spawn Enemies`))
              (:`2`
                (goto _label_5))))
          (:`5`
            (goto _label_4)))
        ;[1 1 1] Reset the attack cooldown and the accumulator
        (set `self.AttackCooldown` (+ (`KismetSystemLibrary.GetGameTimeInSeconds`) 5.0))
        (set `self.AttackIndex(Accumulator)` (+ (`self.AttackIndex(Accumulator)`) 1))))))

(event `self.ReceiveTick`
  (params (DeltaSeconds :type "Float (single-precision)"))
  (`self.FindPlayer`)
  (`self.Attack`))

(event `Check for death`
  ;[1 1 1] Handle damage and death
  (if (<= (`self.Health`) 0.0)
    (`self.K2_DestroyActor`)))

(event `Melee Attack`
  ;[1 1 1] Handle Melee
  (if (>= (`self.GetDistanceTo` (`self.TargetPlayer`)) (`self.MeleeAttackDistance`))
    (`AIBlueprintHelperLibrary.SimpleMoveToLocation` (`self.GetController`) (`self.K2_GetActorLocation` (`self.TargetPlayer`)))
    (else
      (`GameplayStatics.ApplyDamage` (`self.TargetPlayer`) 10.0))))

(event `self.ReceiveAnyDamage`
  (params (Damage :type "Float (single-precision)") (DamageType :type "DamageType Object Reference") (InstigatedBy :type "Controller Object Reference") (DamageCauser :type "Actor Object Reference"))
  ;[1 1 1] Handle damage and death
  (set `self.Health` (- (`self.Health`) Damage))
  (`self.Check for death`))

(event `Ranged Attack`
  ;[1 1 1] Handle Ranged Attack
  (if (>= (`self.GetDistanceTo` (`self.TargetPlayer`)) (`self.MeleeAttackDistance`))
    (`AIBlueprintHelperLibrary.SimpleMoveToLocation` (`self.GetController`) (`self.K2_GetActorLocation` (`self.TargetPlayer`)))
    (else
      (`GameplayStatics.ApplyDamage` (`self.TargetPlayer`) 10.0))))

(event `Spawn Enemies`
  (bind (_returnvalue_x _returnvalue_y _returnvalue_z) (`KismetMathLibrary.BreakVector` (`self.K2_GetActorLocation`)))
  (bind _returnvalue (`KismetMathLibrary.RandomFloatInRange` -500.0 500.0))
  (bind _returnvalue_2 (+ _returnvalue_x _returnvalue))
  (bind _returnvalue_3 (+ _returnvalue_y _returnvalue))
  ;[1 1 1] Handle spawning of minions
  (`|ExecutionSequence`
    (:`then_0`
      (`|SpawnActorFromClass` "/Game/Enemies/BP_Enemy_Mellee.BP_Enemy_Mellee_C" (`KismetMathLibrary.MakeTransform` (`KismetMathLibrary.MakeVector` _returnvalue_2 _returnvalue_3 _returnvalue_z)) "Undefined" "MultiplyWithRoot" null null))
    (:`then_1`
      (`|SpawnActorFromClass` "/Game/Enemies/BP_Enemy_Ranged.BP_Enemy_Ranged_C" (`KismetMathLibrary.MakeTransform` (`KismetMathLibrary.MakeVector` _returnvalue_2 _returnvalue_3 _returnvalue_z)) "Undefined" "MultiplyWithRoot" null null))
    (:`then_2`
      (`|SpawnActorFromClass` "/Game/Enemies/BP_Enemy_Flying.BP_Enemy_Flying_C" (`KismetMathLibrary.MakeTransform` (`KismetMathLibrary.MakeVector` _returnvalue_2 _returnvalue_3 _returnvalue_z)) "Undefined" "MultiplyWithRoot" null null))))

(fn `FindPlayer`
  (`/Engine/EditorBlueprintResources/StandardMacros.IsValid` (`self.TargetPlayer`)
    (:`Is Not Valid`
      (bind _outactors (`GameplayStatics.GetAllActorsOfClass` "/Game/Player_Character/BP_Player0.BP_Player0_C"))
      (set `self.TargetPlayer` (`|GetArrayItem` _outactors)))))

(fn `UserConstructionScript`)